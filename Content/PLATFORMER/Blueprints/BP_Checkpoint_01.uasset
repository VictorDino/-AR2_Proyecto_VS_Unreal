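; BP_Checkpoint_01 is a platformer checkpoint that updates the spawn location of BP_Bunny when it overlaps the checkpoint's box.
; A DoOnce lets only the first bunny overlap copy the checkpoint's SpawnLocation to the bunny and show a WB_Checkpoint widget for a short delay.
; An unconnected node to move the Arrow component to SpawnLocation never runs.
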(event `self.Box.OnComponentBeginOverlap`
  (params (OverlappedComponent :type "PrimitiveComponent Object Reference") (OtherActor :type "Actor Object Reference") (OtherComp :type "PrimitiveComponent Object Reference") (OtherBodyIndex :type Integer) (bFromSweep :type Boolean) (SweepResult :type "HitResult Structure (by ref)"))
  (bind _asbp_bunny (cast `/Game/ThirdPerson/Blueprints/BP_Bunny` OtherActor))
  (`/Engine/EditorBlueprintResources/StandardMacros.DoOnce` false
    (:`Completed`
      (set `/Game/ThirdPerson/Blueprints/BP_Bunny.Spawn Location` (`self.Spawn Location`) _asbp_bunny)
      (bind _returnvalue (`|CreateWidget` "/Game/ThirdPerson/Widget/WB_Checkpoint.WB_Checkpoint_C"))
      (`UserWidget.AddToViewport` _returnvalue 0)
      (`KismetSystemLibrary.Delay` 1.5)
      (`Widget.RemoveFromParent` _returnvalue))))

(fn `UserConstructionScript`)