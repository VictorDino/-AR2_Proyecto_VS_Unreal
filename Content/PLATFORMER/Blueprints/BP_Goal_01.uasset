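; BP_Goal_01 is a platformer level goal that completes the stage when BP_Bunny overlaps its Box trigger.
; It copies the bunny's Coins into CoinsCollected, removes the bunny's MainHUD and shows a WB_StageComplete widget.
; It then switches input to UI only with a visible mouse cursor and pauses the game after a short delay.
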(event `self.Box.OnComponentBeginOverlap`
  (params (OverlappedComponent :type "PrimitiveComponent Object Reference") (OtherActor :type "Actor Object Reference") (OtherComp :type "PrimitiveComponent Object Reference") (OtherBodyIndex :type Integer) (bFromSweep :type Boolean) (SweepResult :type "HitResult Structure (by ref)"))
  (bind _returnvalue (`GameplayStatics.GetPlayerController` 0))
  (bind _asbp_bunny (cast `/Game/ThirdPerson/Blueprints/BP_Bunny` OtherActor))
  (set `/Game/ThirdPerson/Blueprints/BP_Bunny.Coins Collected` (`/Game/ThirdPerson/Blueprints/BP_Bunny.Coins` _asbp_bunny) _asbp_bunny)
  (`Widget.RemoveFromParent` (`/Game/ThirdPerson/Blueprints/BP_Bunny.Main HUD` _asbp_bunny))
  (bind _returnvalue_2 (`|CreateWidget` "/Game/ThirdPerson/Widget/WB_StageComplete.WB_StageComplete_C"))
  (`UserWidget.AddToViewport` _returnvalue_2 0)
  (`WidgetBlueprintLibrary.SetInputMode_UIOnlyEx` _returnvalue null)
  (set `PlayerController.bShowMouseCursor` true _returnvalue)
  (`KismetSystemLibrary.Delay` 1.0)
  (`GameplayStatics.SetGamePaused` true))

(fn `UserConstructionScript`)