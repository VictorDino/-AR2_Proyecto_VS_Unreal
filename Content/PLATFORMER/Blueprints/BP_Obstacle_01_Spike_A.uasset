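; BP_Obstacle_01_Spike_A is a platformer spike trap that rises on overlap and damages characters.
; Overlapping Box plays a timeline lerping the spike between down and up positions; leaving reverses it after a delay.
; SpikeDMG overlaps send BI_Character damage and play a sound, gated by a DoOnce that resets when the timeline finishes.
; The construction script applies configurable meshes and a shared material to the spike and base.
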(event `self.Box.OnComponentBeginOverlap`
  (params (OverlappedComponent :type "PrimitiveComponent Object Reference") (OtherActor :type "Actor Object Reference") (OtherComp :type "PrimitiveComponent Object Reference") (OtherBodyIndex :type Integer) (bFromSweep :type Boolean) (SweepResult :type "HitResult Structure (by ref)"))
  (bind (_direction _newtrack_0) (`Timeline|Spike_` :!label _label)
    (:`Update`
      (`SceneComponent.K2_SetRelativeLocation` (`self.Spike`) (`KismetMathLibrary.VLerp` (`KismetMathLibrary.MakeVector` 0.0 0.0 (`self.Spike Down`)) (`KismetMathLibrary.MakeVector` 0.0 0.0 (`self.Spike Up`)) _newtrack_0) false false))
    (:`Finished`
      (goto _label_2 :!via `Reset`))))

(event `self.Box.OnComponentEndOverlap`
  (params (OverlappedComponent :type "PrimitiveComponent Object Reference") (OtherActor :type "Actor Object Reference") (OtherComp :type "PrimitiveComponent Object Reference") (OtherBodyIndex :type Integer))
  (`KismetSystemLibrary.Delay` 1.0)
  (goto _label :!via `Reverse`))

(event `self.SpikeDMG.OnComponentBeginOverlap`
  (params (OverlappedComponent :type "PrimitiveComponent Object Reference") (OtherActor :type "Actor Object Reference") (OtherComp :type "PrimitiveComponent Object Reference") (OtherBodyIndex :type Integer) (bFromSweep :type Boolean) (SweepResult :type "HitResult Structure (by ref)"))
  (bind _ascharacter (cast `Character` OtherActor))
  (if (`KismetSystemLibrary.DoesImplementInterface` _ascharacter "/Game/ThirdPerson/Interface/BI_Character.BI_Character_C")
    (`/Engine/EditorBlueprintResources/StandardMacros.DoOnce` false :!label _label_2
      (:`Completed`
        (message `/Game/ThirdPerson/Interface/BI_Character.Take Damage Spike` _ascharacter 1)
        (`GameplayStatics.PlaySound2D` "/Game/Other/Wav/Damage_Cue.Damage_Cue" 1.0 1.0 0.0 null null)))))

(fn `UserConstructionScript`
  (`PrimitiveComponent.SetMaterial` (`self.Spike`) 0 (`self.Material`))
  (`PrimitiveComponent.SetMaterial` (`self.Base`) 0 (`self.Material`))
  (`StaticMeshComponent.SetStaticMesh` (`self.Spike`) (`self.Static Mesh Spike`))
  (`StaticMeshComponent.SetStaticMesh` (`self.Base`) (`self.Static Mesh Base`)))